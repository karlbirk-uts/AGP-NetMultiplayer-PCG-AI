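; BP_EnemyCharacter is an enemy character Blueprint that handles the visual display of its equipped gun.
; The EquipWeaponGraphical event sets the gun mesh's visibility, then switches on weapon rarity to choose a Common, Rare, Master or Legendary material instance.
; SetWeaponMaterial applies that instance as the gun mesh's overlay material, tinting it by rarity without replacing its base materials.
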(event EventBeginPlay)

(event Collision|EventActorBeginOverlap
  (params (OtherActor :type Actor%20Object%20Reference)))

(event EventTick
  (params (DeltaSeconds :type Float%20%28single-precision%29)))

(event EventEquipWeaponGraphical
  (params (bIsWeaponVisible :type Boolean) (WeaponRarity :type EWeaponRarity%20Enum :default "Common"))
  (Rendering|SetVisibility (Variables|Default|GetGunMesh) bIsWeaponVisible false)
  (if true
    (switch Utilities|FlowControl|Switch|SwitchonEWeaponRarity WeaponRarity
      (:Common
        (Utilities|SetWeaponMaterial "/Game/Materials/WeaponPickup/MI_Common.MI_Common"))
      (:Rare
        (Utilities|SetWeaponMaterial "/Game/Materials/WeaponPickup/MI_Rare.MI_Rare"))
      (:Master
        (Utilities|SetWeaponMaterial "/Game/Materials/WeaponPickup/MI_Master.MI_Master"))
      (:Legendary
        (Utilities|SetWeaponMaterial "/Game/Materials/WeaponPickup/MI_Legendary.MI_Legendary")))))

(fn ConstructionScript)